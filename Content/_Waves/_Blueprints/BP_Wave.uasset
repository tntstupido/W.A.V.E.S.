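; BP_Wave is a wave actor whose mesh color reflects the frequency in its Spec.
; BeginPlay creates a dynamic material instance on the mesh, and the OnFrequencyChangedBP event triggers a color update.
; The update looks up the frequency in the BP_GM_Waves game mode's color set, prints the matched frequency for debugging and sets the material's BaseColor parameter.
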(event `self.ReceiveBeginPlay`
  (`|ExecutionSequence`
    (:`then_0`
      (bind _returnvalue (`PrimitiveComponent.CreateDynamicMaterialInstance` (`self.Mesh`) 0 null "None"))
      (set `self.WaveDMI` _returnvalue))))

(event `self.OnFrequencyChanged_BP`
  (`self.UpdateWaveColor`))

(fn `UpdateWaveColor`
  (`self.WaveDMI`
    (:`then`
      (bind _asbp_gm_waves (cast `/Game/_Waves/_Blueprints/BP_GM_Waves` (`GameplayStatics.GetGameMode`)))
      (bind (_displayname _frequency _color) (break `WaveColorDef` (`DA_WaveColorSet.FindByFrequency` (`GM_Waves.GetColorSet` _asbp_gm_waves) (`.Frequency` (break `WaveSpec` (`self.Spec`))))))
      (`KismetSystemLibrary.PrintString` (`|GetEnumeratorNameAsString` _frequency))
      (`MaterialInstanceDynamic.SetVectorParameterValue` (`self.WaveDMI`) "BaseColor" _color))
    (:`else`)))

(fn `UserConstructionScript`)